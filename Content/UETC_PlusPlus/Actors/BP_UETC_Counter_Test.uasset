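; BP_UETC_Counter_Test is a test actor that displays a counting number through a text render component.
; BeginPlay sets the counter variable to ten and writes it to the text.
; Every Tick decrements the variable by one and refreshes the text, so the count falls per frame with no lower bound or time scaling.
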(event `self.ReceiveBeginPlay`
  (bind _output_get (set `self.TextVariable` 10))
  (`TextRenderComponent.K2_SetText` (`self.TextRender`) (`KismetTextLibrary.Conv_IntToText` _output_get)))

(event `self.ReceiveTick`
  (params (DeltaSeconds :type "Float (single-precision)"))
  (bind _output_get (set `self.TextVariable` (- (`self.TextVariable`) 1)))
  (`TextRenderComponent.K2_SetText` (`self.TextRender`) (`KismetTextLibrary.Conv_IntToText` _output_get)))

(fn `UserConstructionScript`)